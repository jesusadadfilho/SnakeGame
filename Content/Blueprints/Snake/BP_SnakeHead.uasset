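; Snake player actor for a grid-based Snake game, stepping the head 100 units along its direction on a looping 0.1-second timer.
; Each step records child component positions, then moves every body part into its predecessor's previous spot.
; Direction changes reject reversals, and growth attaches spawned BP_SnakeBodyPart actors to the root.
; Wall hits wrap the head 3000 units backward; death simply reopens SnakeMap, marked as a to-do.
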(event Custom|UpdateDirection
  (params (NewDirection :type EN_Directions%20Enum :default "NewEnumerator0") (Value :type Vector%202D%20Structure))
  (switch Utilities|FlowControl|Switch|SwitchonEN_Directions NewDirection
    (:NewEnumerator0
      (if (Utilities|Enum|NotEqual(Enum) (Variables|Default|GetLastDiretion) "NewEnumerator1")
        (Variables|Default|SetDirection Value)
        (Variables|Default|SetLastDiretion NewDirection)))
    (:NewEnumerator1
      (if (Utilities|Enum|NotEqual(Enum) (Variables|Default|GetLastDiretion) "NewEnumerator0")
        (Variables|Default|SetDirection Value)
        (Variables|Default|SetLastDiretion NewDirection)))
    (:NewEnumerator2
      (if (Utilities|Enum|NotEqual(Enum) (Variables|Default|GetLastDiretion) "NewEnumerator3")
        (Variables|Default|SetDirection Value)
        (Variables|Default|SetLastDiretion NewDirection)))
    (:NewEnumerator3
      (if (Utilities|Enum|NotEqual(Enum) (Variables|Default|GetLastDiretion) "NewEnumerator2")
        (Variables|Default|SetDirection Value)
        (Variables|Default|SetLastDiretion NewDirection)))))

(event Custom|UpdateSnakePosition
  (bind _defaultsceneroot (Variables|Default|GetDefaultSceneRoot))
  (bind _children (Components|GetChildrenComponents _defaultsceneroot false))
  (Utilities|Array|Clear (Variables|Default|GetPositions))
  (for (_array_element _array_index) _children
    (if (!= _array_index (- (Utilities|Array|Length _children) 1))
      (Utilities|Array|Add (Variables|Default|GetPositions) (Transformation|GetWorldLocation _array_element))))
  (CallFunction|MoveSnakeHead)
  (if (> (Utilities|Array|Length (Components|GetChildrenComponents (Variables|Default|GetDefaultSceneRoot) false)) 1)
    (CallFunction|MoveSnakeBodyParts)))

(event Custom|IncreaseSnake
  (bind _returnvalue (Game|SpawnActorfromClass "/Game/Blueprints/Snake/BP_SnakeBodyPart.BP_SnakeBodyPart_C" (Math|Transform|MakeTransform "0.000000, 0,0.000000" "0, 0, 0" "1.000000,1,1") "Undefined" 0 0))
  (Transformation|AttachComponentToComponent _returnvalue (Variables|Default|GetDefaultSceneRoot) "None" "KeepRelative" "KeepRelative" "KeepRelative" true))

(event Custom|MoveSnakeHead
  (bind _direction (Variables|Default|GetDirection))
  (bind _head (Variables|Default|GetHead))
  (bind _returnvalue (Transformation|GetWorldLocation _head))
  (bind (_x _y) (Math|Vector2D|BreakVector2D _direction))
  (bind (_x_2 _y_2 _z) (Math|Vector|BreakVector _returnvalue))
  (Transformation|SetWorldLocation (Variables|Default|GetHead) (Math|Vector|MakeVector (+ (* _x 1e+02) _x_2) (+ (* _y 1e+02) _y_2) _z) false false))

(event Custom|MoveSnakeBodyParts
  (for (_array_element _array_index) (Components|GetChildrenComponents (Variables|Default|GetDefaultSceneRoot) false)
    (if (!= _array_index 0)
      (Transformation|SetWorldLocation _array_element (Utilities|Array|Get(acopy) (Variables|Default|GetPositions) (- _array_index 1)) false false))))

(event Custom|Death
  ;[1 1 1] @ToDo- make snake death
  (Game|OpenLevel(byName) "SnakeMap"))

(event Custom|HitWall
  (bind _direction (Variables|Default|GetDirection))
  (bind _head (Variables|Default|GetHead))
  (bind (_x _y) (Math|Vector2D|BreakVector2D _direction))
  (bind _returnvalue (Transformation|GetWorldLocation _head))
  (bind (_x_2 _y_2 _z) (Math|Vector|BreakVector _returnvalue))
  (Transformation|SetWorldLocation (Variables|Default|GetHead) (Math|Vector|MakeVector (+ (* _x -3e+03) _x_2) (+ _y_2 (* _y -3e+03)) _z) false false))

(event EventBeginPlay
  (Utilities|Time|SetTimerbyEvent (delegate Custom|UpdateSnakePosition) 0.1 true))

(event Collision|EventActorBeginOverlap
  (params (OtherActor :type Actor%20Object%20Reference)))

(event EventTick
  (params (DeltaSeconds :type Float%20%28single-precision%29)))

(fn ConstructionScript)