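; Player controller for a Snake game that steers the snake head from player input.
; Four input actions for left, right, up and down each look up BP_SnakeHead with GetActorOfClass on every press.
; Each then calls UpdateDirection on it, passing a direction enum and a matching 2D unit vector.
; The controller holds no other logic.
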(event EventBeginPlay)

(event EventTick
  (params (DeltaSeconds :type Float%20%28single-precision%29)))

(event Input|ActionEvents|InputActionGoLeft
  (params (Key :type Key%20Structure :default "None"))
  (:Pressed
    (bind _returnvalue (Actor|GetActorOfClass "/Game/Blueprints/Snake/BP_SnakeHead.BP_SnakeHead_C"))
    (Default|UpdateDirection _returnvalue "NewEnumerator1" "(X=0.000000,Y=-1.000000)")))

(event Input|ActionEvents|InputActionGoRight
  (params (Key :type Key%20Structure :default "None"))
  (:Pressed
    (bind _returnvalue (Actor|GetActorOfClass "/Game/Blueprints/Snake/BP_SnakeHead.BP_SnakeHead_C"))
    (Default|UpdateDirection _returnvalue "NewEnumerator0" "(X=0.000000,Y=1.000000)")))

(event Input|ActionEvents|InputActionGoUp
  (params (Key :type Key%20Structure :default "None"))
  (:Pressed
    (bind _returnvalue (Actor|GetActorOfClass "/Game/Blueprints/Snake/BP_SnakeHead.BP_SnakeHead_C"))
    (Default|UpdateDirection _returnvalue "NewEnumerator2" "(X=1.000000,Y=0.000000)")))

(event Input|ActionEvents|InputActionGoDown
  (params (Key :type Key%20Structure :default "None"))
  (:Pressed
    (bind _returnvalue (Actor|GetActorOfClass "/Game/Blueprints/Snake/BP_SnakeHead.BP_SnakeHead_C"))
    (Default|UpdateDirection _returnvalue "NewEnumerator3" "(X=-1.000000,Y=0.000000)")))

(fn ConstructionScript)