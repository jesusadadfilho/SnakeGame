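; Food pickup for a Snake game that grows the snake when BP_SnakeHead overlaps its box, then moves itself to a new grid cell.
; SpawnFood runs on BeginPlay and after each pickup, picking random cells on a fixed-height grid and calling itself recursively on a match with the head or a body part.
; Each check and the final move roll separate random positions, so the food can still land on the snake.
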(event OnComponentBeginOverlap(Box)
  (params (OverlappedComponent :type Primitive%20Component%20Object%20Reference) (OtherActor :type Actor%20Object%20Reference) (OtherComp :type Primitive%20Component%20Object%20Reference) (OtherBodyIndex :type Integer) (bFromSweep :type Boolean) (SweepResult :type Hit%20Result%20Structure%20%28by%20ref%29))
  (bind _asbp_snake_head (Utilities|Casting|CastToBP_SnakeHead OtherActor))
  (Default|IncreaseSnake _asbp_snake_head)
  (CallFunction|SpawnFood))

(event Custom|SpawnFood
  (bind _returnvalue (Math|Random|RandomIntegerinRange 0 28))
  (bind _returnvalue_2 (Math|Random|RandomIntegerinRange 0 28))
  (bind _returnvalue_3 (* _returnvalue 100))
  (bind _returnvalue_4 (* _returnvalue_2 100))
  (bind _returnvalue_5 (- 1450 _returnvalue_3))
  (bind _returnvalue_6 (- 1450 _returnvalue_4))
  (bind _returnvalue_7 (Math|Conversions|ToFloat(Integer) _returnvalue_6))
  (bind _returnvalue_8 (Math|Conversions|ToFloat(Integer) _returnvalue_5))
  (bind _returnvalue_9 (Math|Vector|MakeVector _returnvalue_7 _returnvalue_8 1e+02))
  (bind _returnvalue_10 (Actor|GetActorOfClass "/Game/Blueprints/Snake/BP_SnakeHead.BP_SnakeHead_C"))
  (if (Class|KismetMathLibrary|EqualExactlyVectorVector (Transformation|GetWorldLocation (Variables|/Game/Blueprints/Snake/BP_SnakeHead.BP_SnakeHead_C|GetHead _returnvalue_10)) _returnvalue_9)
    (CallFunction|SpawnFood)
    (else
      (bind _outactors (Actor|GetAllActorsOfClass "/Game/Blueprints/Snake/BP_SnakeBodyPart.BP_SnakeBodyPart_C"))
      (for _array_element _outactors
        (if (Class|KismetMathLibrary|EqualExactlyVectorVector (Transformation|GetActorLocation _array_element) _returnvalue_9)
          (CallFunction|SpawnFood)))
      (Transformation|SetActorLocation _returnvalue_9 false false))))

(event EventBeginPlay
  (CallFunction|SpawnFood))

(event EventTick
  (params (DeltaSeconds :type Float%20%28single-precision%29)))

(fn ConstructionScript)